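; Game coordinator actor that spawns weapon loot and handles the music change at game over.
; LootSpawner loops indefinitely, spawning a random class from Weapons at a random reachable navmesh point around the actor, with a short random delay between spawns.
; EndGame fades out the in-game music, then spawns and fades in the game-over cue.
; Both are custom events, with no caller in this Blueprint.
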(event Custom|Loot%20Spawner
  (bind _weapons (Variables|Default|GetWeapons))
  ;[0 0 0] Loot Spawner
  (Game|SpawnActorfromClass (Utilities|Array|Get(acopy) _weapons (Math|Random|RandomInteger (Utilities|Array|Length _weapons))) (Math|Transform|MakeTransform (.RandomLocation (AI|Navigation|GetRandomReachablePointinRadius (Transformation|GetActorLocation) 99999.0 0 0)) "0, 0, 0" "1,1,1") "Undefined" 0 true 0 :!label _label)
  (Utilities|FlowControl|Delay (Math|Random|RandomFloatinRange 3.0 5.0))
  (goto _label))

(event Custom|End%20Game
  ;[0 0 0] End Game
  (Audio|Components|Audio|FadeOut (Variables|Default|GetDuring%20Game%20Music) 1.0 0.0 "Linear" :!class /Script/Engine.AudioComponent) ; Fade out During Game Music
  (bind _returnvalue (Audio|SpawnSound2D "/Game/Downloaded/Sounds/Music/Cue_Gameover.Cue_Gameover" 1.0 1.0 0.0 0)) ; Spawn And Play Death Music
  (Audio|Components|Audio|FadeIn _returnvalue 2.0 1.0 0.0 "Linear" :!class /Script/Engine.AudioComponent) ; Fade In Death Music
)

(fn ConstructionScript)