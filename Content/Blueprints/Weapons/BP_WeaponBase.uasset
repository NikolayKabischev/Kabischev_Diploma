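; Base weapon Blueprint that handles single-shot or automatic projectile firing with ammo tracking.
; BeginFiring fires at once and, when FireRate is positive, starts a looping timer that StopFiring or an empty magazine clears.
; Fire checks CanFire and ammo, broadcasts the ammo change, then spawns a damage-carrying projectile at the muzzle with random yaw spread.
; OnFired adds muzzle flash, 2D sound and Timeline-driven recoil rotation on the weapon mesh.
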(event Custom|Fire
  (bind _muzzletransform (Variables|Default|GetMuzzleTransform))
  (bind _weapon_spread (Variables|Properties|GetWeapon%20Spread))
  (bind _returnvalue (Transformation|GetWorldTransform _muzzletransform))
  ;[0 0 0] Shooting
  ;;[1 0 1] Shooting Loop
  (if (Variables|Default|GetCan%20Fire)
    (if (> (Variables|Properties|GetAmmo) 0) ; Have Ammo?
      (bind _result (Math|Integer|DecrementInt (Variables|Properties|GetAmmo))
        (:%20%20
          (Default|CallOnAmmoChanged _result) ; Update Ammo on Widget
          (Game|SpawnActorfromClass (Variables|Properties|GetProjectile) (Math|Transform|MakeTransform (.location _returnvalue) (Math|Rotator|MakeRotator (.roll (.rotation _returnvalue)) (.pitch (.rotation _returnvalue)) (+ (.yaw (.rotation _returnvalue)) (Math|Random|RandomFloatinRange (* _weapon_spread -1.0) _weapon_spread))) (.scale _returnvalue)) "AlwaysSpawn" 0 (Variables|Properties|GetDamage) 0) ; Spawn Projectile
          (CallFunction|OnFired)))
      (else
        (CallFunction|StopFiring)))))

(event Custom|Begin%20Firing
  ;[0 0 0] Shooting
  ;;[1 0 1] Start Shooting
  (if (> (Variables|Properties|GetFire%20Rate) 0.0) ; Is Automatic Weapon?
    (Utilities|Time|SetTimerbyFunctionName 0 "Fire" (Variables|Properties|GetFire%20Rate) true) ; Begin Shooting Loop
    (CallFunction|Fire)
    (else
      (CallFunction|Fire))))

(event Custom|Stop%20Firing
  ;[0 0 0] Shooting
  ;;[1 0 1] Stop Shooting
  (Utilities|Time|ClearTimerbyFunctionName 0 "Fire") ; Stop Shooting Loop
)

(event Custom|On%20Fired
  ;[0 0 0] Shooting
  ;;[1 0 1] On Shot
  (Effects|SpawnEmitterAttached 0 (Variables|Default|GetMuzzleFX) "None" "0, 0, 0" (Variables|/Script/Engine.SceneComponent|GetRelativeRotation (Variables|Default|GetMuzzleFX)) "1.000000,1.000000,1.000000" "SnapToTarget") ; Spawn Muzzle Flash
  (Audio|SpawnSound2D 0 1.0 1.0 0.0 0) ; Spawn Shot Sound
  ;;;[1 0 0] Recoil
  (bind _newtrack_0 (Timeline|Recoil PlayFromStart) ; Add Recoil
    (:Update
      (Transformation|SetRelativeRotation (Variables|Default|GetWeapon%20Mesh) (Math|Rotator|MakeRotator (Math|Float|Lerp 0.0 -15.0 _newtrack_0) 0.0 0.0) false false))))

(fn ConstructionScript)