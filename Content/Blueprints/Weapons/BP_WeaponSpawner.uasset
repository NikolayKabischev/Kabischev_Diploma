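; BP_WeaponSpawner is a rotating weapon pickup that arms the player on overlap and can optionally destroy itself after a delay.
; Its per-tick spin scales with global time dilation, so it slows during slow motion.
; On overlap it replaces the held weapon with a copy of its child actor's class, lerped from the pickup to the hand.
; It then calls StartGame on BP_GameCoordinator, updates the HUD, plays a sound and destroys itself.
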(event OnComponentBeginOverlap(Sphere)
  (params (OverlappedComponent :type Primitive%20Component%20Object%20Reference) (OtherActor :type Actor%20Object%20Reference) (OtherComp :type Primitive%20Component%20Object%20Reference) (OtherBodyIndex :type Integer) (bFromSweep :type Boolean) (SweepResult :type Hit%20Result%20Structure%20%28by%20ref%29))
  ;[0 0 0] Give Player Weapon
  (bind _asthird_person_character (Utilities|Casting|CastToThirdPersonCharacter OtherActor))
  ;;[1 0 0 1 15] Destroy Current Weapon The Player Is Holding
  (bind _weapon (Variables|/Game/Blueprints/ThirdPersonCharacter.ThirdPersonCharacter_C|GetWeapon _asthird_person_character)
    (:then
      (Actor|DestroyActor _weapon))
    (:else
      _))
  (bind _returnvalue (AddComponent|AddChildActorComponent _asthird_person_character true (Transformation|GetWorldTransform (Variables|Default|GetChildActor)))) ; Add Weapon Component
  (ChildActorComponent|SetChildActorClass _returnvalue (Variables|/Script/Engine.ChildActorComponent|GetChildActorClass (Variables|Default|GetChildActor))) ; Set Weapon
  (Transformation|AttachComponentToComponent _returnvalue (Variables|/Game/Blueprints/ThirdPersonCharacter.ThirdPersonCharacter_C|GetWeapon1%20Pos _asthird_person_character) "None" "KeepWorld" "KeepWorld" "KeepWorld" true) ; Attach Weapon To Player Hand
  (bind _asbp_weapon_base (Utilities|Casting|CastToBP_WeaponBase (Variables|/Script/Engine.ChildActorComponent|GetChildActor _returnvalue)))
  (bind _asthird_person_character_2 (Utilities|Casting|CastToThirdPersonCharacter (Game|GetPlayerCharacter 0)))
  (Variables|/Game/Blueprints/ThirdPersonCharacter.ThirdPersonCharacter_C|SetWeapon _asthird_person_character_2 _asbp_weapon_base)
  (Default|LerpWeapon _asthird_person_character_2) ; Smoothly Move Weapon To Player Hand
  (bind _outactors (Actor|GetAllActorsOfClass "/Game/Blueprints/BP_GameCoordinator.BP_GameCoordinator_C"))
  (Default|StartGame (Utilities|Array|Get(acopy) _outactors)) ; Start Game If Its not Started
  (Default|NewWeapon (Variables|/Game/UI/InGame/UI_InGame.UI_InGame_C|GetUI_InGame_DuringGame (Variables|/Game/UI/UI_Main.UI_Main_C|GetUI_InGame (Variables|/Game/Blueprints/ThirdPersonCharacter.ThirdPersonCharacter_C|GetUI%20Main _asthird_person_character_2)))) ; Tell During Game Widget That The Player Has a New Weapon
  (Audio|PlaySound2D 0 1.0 1.0 0.0 0 0) ; Play Equip Sound
  (Actor|DestroyActor))

(event EventTick
  (params (DeltaSeconds :type Float%20%28single-precision%29))
  ;[0 0 0] Rotate
  (Transformation|AddActorLocalRotation (Math|Rotator|MakeRotator 0.0 0.0 (Class|GameplayStatics|GetGlobalTimeDilation)) false false))

(event EventBeginPlay
  ;[0 0 0] Spawned
  (if (Variables|Default|GetTimed%20Destroy?) ; Should Destroy After Some Time?
    (Utilities|FlowControl|Delay 1e+01)
    (Actor|DestroyActor)))

(fn ConstructionScript)