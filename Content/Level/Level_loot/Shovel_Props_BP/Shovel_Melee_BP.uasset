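; Shovel melee pickup placed as level loot that equips the player with a shovel and raises their minimum damage.
; When the player character overlaps its sphere, it shows the character's Shovel component, plays a gold sparkle effect, destroys itself and adds the damage buff to DamageMin.
; A second sequence branch opens a shovel tutorial widget, pauses the game and switches input to UI only.
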(event OnComponentBeginOverlap(Sphere)
  (params (OverlappedComponent :type Primitive%20Component%20Object%20Reference) (OtherActor :type Actor%20Object%20Reference) (OtherComp :type Primitive%20Component%20Object%20Reference) (OtherBodyIndex :type Integer) (bFromSweep :type Boolean) (SweepResult :type Hit%20Result%20Structure%20%28by%20ref%29))
  (bind _returnvalue (Game|GetPlayerCharacter 0))
  (bind _astop_down_character (Utilities|Casting|CastToTopDownCharacter _returnvalue))
  (if (== OtherActor (Game|GetPlayerCharacter 0))
    (Utilities|FlowControl|Sequence
      (:then_0
        (bind _astop_down_character_2 (Utilities|Casting|CastToTopDownCharacter OtherActor))
        (Rendering|SetVisibility (Variables|/Game/TopDownBP/Main_BP/TopDownCharacter.TopDownCharacter_C|GetShovel _astop_down_character_2) true false)
        (Effects|SpawnEmitteratLocation "/Game/Downloaded/InfinityBladeEffects/Effects/FX_Treasure/Gold_Bag/P_GoldSparkle_Bag_Pickup.P_GoldSparkle_Bag_Pickup" (Transformation|GetWorldLocation (Variables|Default|GetStaticMesh)) "0, 0, 0" "2.000000,2.000000,2.000000")
        (Actor|DestroyActor)
        (Variables|/Game/TopDownBP/Main_BP/TopDownCharacter.TopDownCharacter_C|SetDamage_min _astop_down_character (+ (Variables|/Game/TopDownBP/Main_BP/TopDownCharacter.TopDownCharacter_C|GetDamage_min _astop_down_character) (Variables|Default|GetShovel_Base_Damage_Buff))))
      (:then_1
        (bind _returnvalue_2 (UserInterface|CreateWidget "/Game/UI/Tutorial/Shovel/W_Shovel_tutor_widget.W_Shovel_tutor_widget_C" (Game|GetPlayerController 0)))
        (UserInterface|Viewport|AddtoViewport _returnvalue_2 0)
        (Game|SetGamePaused true)
        (Input|SetInputModeUIOnly (Game|GetPlayerController 0) _returnvalue_2 "DoNotLock")))))

(event EventBeginPlay)

(event Collision|EventActorBeginOverlap
  (params (OtherActor :type Actor%20Object%20Reference)))

(event EventTick
  (params (DeltaSeconds :type Float%20%28single-precision%29)))

(fn ConstructionScript)