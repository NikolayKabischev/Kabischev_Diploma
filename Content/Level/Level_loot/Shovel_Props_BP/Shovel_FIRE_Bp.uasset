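; Fire shovel pickup that enables the player's fire shovel when TopDownCharacter overlaps its sphere.
; The overlap sets ShovelFireON on the character, spawns a gold sparkle emitter at the mesh and destroys the actor.
; A DoOnce after the destroy shows the fire shovel tutorial widget and switches input to UI only, with game pause explicitly set to false.
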(event OnComponentBeginOverlap(Sphere)
  (params (OverlappedComponent :type Primitive%20Component%20Object%20Reference) (OtherActor :type Actor%20Object%20Reference) (OtherComp :type Primitive%20Component%20Object%20Reference) (OtherBodyIndex :type Integer) (bFromSweep :type Boolean) (SweepResult :type Hit%20Result%20Structure%20%28by%20ref%29))
  (bind _astop_down_character (Utilities|Casting|CastToTopDownCharacter OtherActor))
  (Variables|/Game/TopDownBP/Main_BP/TopDownCharacter.TopDownCharacter_C|SetShovel_Fire_ON _astop_down_character true)
  (Effects|SpawnEmitteratLocation "/Game/Downloaded/InfinityBladeEffects/Effects/FX_Treasure/Gold_Bag/P_GoldSparkle_Bag_Pickup.P_GoldSparkle_Bag_Pickup" (Transformation|GetWorldLocation (Variables|Default|GetStaticMesh)) "0, 0, 0" "2.000000,2.000000,2.000000")
  (Actor|DestroyActor)
  (Utilities|FlowControl|DoOnce false
    (:Completed
      (bind _returnvalue (UserInterface|CreateWidget "/Game/UI/Tutorial/Shovel/W_Shovel_FIREtutor_widget1.W_Shovel_FIREtutor_widget1_C"))
      (UserInterface|Viewport|AddtoViewport _returnvalue 0)
      (Input|SetInputModeUIOnly (Game|GetPlayerController 0) _returnvalue "LockOnCapture")
      (Game|SetGamePaused false))))

(event EventBeginPlay)

(event Collision|EventActorBeginOverlap
  (params (OtherActor :type Actor%20Object%20Reference)))

(event EventTick
  (params (DeltaSeconds :type Float%20%28single-precision%29)))

(fn ConstructionScript)