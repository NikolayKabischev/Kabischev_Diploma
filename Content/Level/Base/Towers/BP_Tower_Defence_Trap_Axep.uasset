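; Buildable axe trap for tower defense that starts hidden and, once visible, damages non-player actors entering its enemy trigger.
; A DoOnce limits it to one victim per cycle: axe particle effect, delayed damage, then effect removal and reset after Duration.
; The player trigger sets IsNearTower and, while the trap is hidden, shows a build or need-gold prompt based on current gold.
; Unhiding the trap is not handled here.
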(event OnComponentBeginOverlap(Trigger_enemy)
  (params (OverlappedComponent :type Primitive%20Component%20Object%20Reference) (OtherActor :type Actor%20Object%20Reference) (OtherComp :type Primitive%20Component%20Object%20Reference) (OtherBodyIndex :type Integer) (bFromSweep :type Boolean) (SweepResult :type Hit%20Result%20Structure%20%28by%20ref%29))
  (if (!= OtherActor (Game|GetPlayerCharacter 0))
    (if (not (Variables|Rendering|GetbHidden self))
      (Utilities|FlowControl|DoOnce false :!label _label
        (:Completed
          (bind _returnvalue (Effects|SpawnEmitteratLocation "/Game/Downloaded/InfinityBladeEffects/Effects/FX_Mobile/Fire/combat/P_YoYo_Fire_Axe_00.P_YoYo_Fire_Axe_00" (+ (Transformation|GetWorldLocation (Variables|Default|GetTrigger_enemy)) "0, 0,50.000000") "0, 0, 0" "2.000000,2.000000,2.000000" false))
          (Utilities|FlowControl|Delay 1.0)
          (Game|Damage|ApplyDamage OtherActor (Variables|Default|GetBase%20Damage) 0 0)
          (Utilities|FlowControl|Delay (Variables|Default|GetDuration))
          (Components|DestroyComponent _returnvalue)
          (goto _label Reset))))))

(event OnComponentBeginOverlap(Trigger_player)
  (params (OverlappedComponent :type Primitive%20Component%20Object%20Reference) (OtherActor :type Actor%20Object%20Reference) (OtherComp :type Primitive%20Component%20Object%20Reference) (OtherBodyIndex :type Integer) (bFromSweep :type Boolean) (SweepResult :type Hit%20Result%20Structure%20%28by%20ref%29))
  (bind _astop_down_character (Utilities|Casting|CastToTopDownCharacter OtherActor))
  (Variables|Default|SetIs_Near_Tower true)
  (if (>= (Variables|/Game/TopDownBP/Main_BP/Status_Health.Status_Health_C|GetCurrentGold (Variables|/Game/TopDownBP/Main_BP/TopDownCharacter.TopDownCharacter_C|GetStatus_health _astop_down_character)) 1e+01)
    (if (Variables|Rendering|GetbHidden)
      (bind _returnvalue (UserInterface|CreateWidget "/Game/UI/Base/W_F_to_build_Tower.W_F_to_build_Tower_C"))
      (UserInterface|Viewport|AddtoViewport _returnvalue 0)
      (else
        (Widget|RemovefromParent (stale _returnvalue_2))))
    (elif (Variables|Rendering|GetbHidden self)
      (bind _returnvalue_2 (UserInterface|CreateWidget "/Game/UI/Base/W_need_10_gold.W_need_10_gold_C"))
      (UserInterface|Viewport|AddtoViewport _returnvalue_2 0))))

(event OnComponentEndOverlap(Trigger_player)
  (params (OverlappedComponent :type Primitive%20Component%20Object%20Reference) (OtherActor :type Actor%20Object%20Reference) (OtherComp :type Primitive%20Component%20Object%20Reference) (OtherBodyIndex :type Integer))
  (Variables|Default|SetIs_Near_Tower false)
  (Widget|RemovefromParent (stale OnComponentBeginOverlap(Trigger_player) _returnvalue_2)))

(event EventBeginPlay
  (Rendering|SetActorHiddenInGame self true))

(fn ConstructionScript)