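; Buildable base health spawner that starts hidden and, while visible, spawns Health_Loot at its Sphere component.
; Tick runs into a two-minute Delay, which acts as the repeating spawn timer.
; While hidden, Box overlap by TopDownCharacter sets IsNearPumpkin and shows a build prompt or a gold-shortage widget, depending on StatusHealth gold.
; Leaving the Box clears both; the unhide and payment logic are outside this Blueprint.
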(event OnComponentBeginOverlap(Box)
  (params (OverlappedComponent :type Primitive%20Component%20Object%20Reference) (OtherActor :type Actor%20Object%20Reference) (OtherComp :type Primitive%20Component%20Object%20Reference) (OtherBodyIndex :type Integer) (bFromSweep :type Boolean) (SweepResult :type Hit%20Result%20Structure%20%28by%20ref%29))
  (bind _astop_down_character (Utilities|Casting|CastToTopDownCharacter OtherActor))
  (Variables|Default|SetIs_Near_Pumpkin true)
  (if (>= (Variables|/Game/TopDownBP/Main_BP/Status_Health.Status_Health_C|GetCurrentGold (Variables|/Game/TopDownBP/Main_BP/TopDownCharacter.TopDownCharacter_C|GetStatus_health _astop_down_character)) 1e+01)
    (if (Variables|Rendering|GetbHidden self)
      (bind _returnvalue (UserInterface|CreateWidget "/Game/UI/Base/W_F_to_build.W_F_to_build_C"))
      (UserInterface|Viewport|AddtoViewport _returnvalue 0)
      (else
        (Widget|RemovefromParent (stale _returnvalue_2))))
    (elif (Variables|Rendering|GetbHidden self)
      (bind _returnvalue_2 (UserInterface|CreateWidget "/Game/UI/Base/W_need_10_gold.W_need_10_gold_C"))
      (UserInterface|Viewport|AddtoViewport _returnvalue_2 0))))

(event OnComponentEndOverlap(Box)
  (params (OverlappedComponent :type Primitive%20Component%20Object%20Reference) (OtherActor :type Actor%20Object%20Reference) (OtherComp :type Primitive%20Component%20Object%20Reference) (OtherBodyIndex :type Integer))
  (Variables|Default|SetIs_Near_Pumpkin false)
  (Widget|RemovefromParent (stale OnComponentBeginOverlap(Box) _returnvalue_2)))

(event EventBeginPlay
  (Rendering|SetActorHiddenInGame true))

(event EventTick
  (params (DeltaSeconds :type Float%20%28single-precision%29))
  (if (not (Variables|Rendering|GetbHidden self))
    (Utilities|FlowControl|Delay 1.2e+02)
    (Game|SpawnActorfromClass "/Game/AI_Enemy/Enemy_Loot/Health_loot/Health_Loot.Health_Loot_C" (Math|Transform|MakeTransform (Transformation|GetWorldLocation (Variables|Default|GetSphere)) "0, 0, 0" "1,1,1") "Undefined" 0 0)))

(fn ConstructionScript)