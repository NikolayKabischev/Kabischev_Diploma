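; Carrot garden bed for the player's base that starts hidden as an unbuilt plot and spawns mana loot.
; Entering the box flags proximity and, while the bed is hidden, shows a build or need-gold prompt based on the character's gold, plus a seeds prompt if no carrot is looted.
; Leaving clears the flag and prompts.
; A separate sphere overlap spawns Mana_loot at the sphere after a delay; building is not handled here.
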(event OnComponentBeginOverlap(Sphere)
  (params (OverlappedComponent :type Primitive%20Component%20Object%20Reference) (OtherActor :type Actor%20Object%20Reference) (OtherComp :type Primitive%20Component%20Object%20Reference) (OtherBodyIndex :type Integer) (bFromSweep :type Boolean) (SweepResult :type Hit%20Result%20Structure%20%28by%20ref%29))
  (Utilities|FlowControl|Delay 3e+01)
  (Game|SpawnActorfromClass "/Game/AI_Enemy/Enemy_Loot/Mana_loot/Mana_loot.Mana_loot_C" (Math|Transform|MakeTransform (Transformation|GetWorldLocation (Variables|Default|GetSphere)) "0, 0, 0" "1,1,1") "Undefined" 0 0))

(event OnComponentBeginOverlap(Box)
  (params (OverlappedComponent :type Primitive%20Component%20Object%20Reference) (OtherActor :type Actor%20Object%20Reference) (OtherComp :type Primitive%20Component%20Object%20Reference) (OtherBodyIndex :type Integer) (bFromSweep :type Boolean) (SweepResult :type Hit%20Result%20Structure%20%28by%20ref%29))
  (bind _astop_down_character (Utilities|Casting|CastToTopDownCharacter OtherActor))
  (Variables|Default|SetIs_Near_Carrots true)
  (if (>= (Variables|/Game/TopDownBP/Main_BP/Status_Health.Status_Health_C|GetCurrentGold (Variables|/Game/TopDownBP/Main_BP/TopDownCharacter.TopDownCharacter_C|GetStatus_health _astop_down_character)) 1e+01)
    (if (Variables|Rendering|GetbHidden self)
      (bind _returnvalue (UserInterface|CreateWidget "/Game/UI/Base/W_F_to_build.W_F_to_build_C"))
      (UserInterface|Viewport|AddtoViewport _returnvalue 0)
      (if (not (Variables|/Game/TopDownBP/Main_BP/TopDownCharacter.TopDownCharacter_C|GetCarrot_looted (.AsTop%20Down%20Character (Utilities|Casting|CastToTopDownCharacter (Game|GetPlayerCharacter 0))))) :!label _label
        (bind _returnvalue_2 (UserInterface|CreateWidget "/Game/UI/Base/Gryadki/W_need_Carrot_Seeds2.W_need_Carrot_Seeds2_C"))
        (UserInterface|Viewport|AddtoViewport _returnvalue_2 0)))
    (elif (Variables|Rendering|GetbHidden self)
      (bind _returnvalue_3 (UserInterface|CreateWidget "/Game/UI/Base/W_need_10_gold.W_need_10_gold_C"))
      (UserInterface|Viewport|AddtoViewport _returnvalue_3 0)
      (goto _label))))

(event OnComponentEndOverlap(Box)
  (params (OverlappedComponent :type Primitive%20Component%20Object%20Reference) (OtherActor :type Actor%20Object%20Reference) (OtherComp :type Primitive%20Component%20Object%20Reference) (OtherBodyIndex :type Integer))
  (Variables|Default|SetIs_Near_Carrots false)
  (Widget|RemovefromParent (stale OnComponentBeginOverlap(Box) _returnvalue_3)))

(event EventBeginPlay
  (Rendering|SetActorHiddenInGame true))

(fn ConstructionScript)