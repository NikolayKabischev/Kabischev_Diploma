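; Base enemy AI Blueprint, apparently a zombie, that turns toward the player on spawn, chases and damages them.
; An AI MoveTo loop applies damage on reaching the player and retries after a short delay.
; Its damage event, also fed by radial damage, lowers its own Health but destroys the player character at zero.
; AnyDamage plays a hit sound or death sequence; mesh cursor events toggle a selection highlight, marked as broken.
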(event OnClicked(Mesh)
  (params (TouchedComponent :type Primitive%20Component%20Object%20Reference) (ButtonPressed :type Key%20Structure :default "None"))
  ;[1 0 0] Выделение меша от наведения курсора (НЕ РАБОТАЕТ ???)
  (Rendering|Material|SetScalarParameterValueonMaterials (Variables|Character|GetMesh) "Enemy_Select" 1.0))

(event OnEndCursorOver(Mesh)
  (params (TouchedComponent :type Primitive%20Component%20Object%20Reference))
  ;[1 0 0] Выделение меша от наведения курсора (НЕ РАБОТАЕТ ???)
  (Rendering|Material|SetScalarParameterValueonMaterials (Variables|Character|GetMesh) "Enemy_Select" 0.0))

(event Custom|Apply%20Damage
  (params (Damage :type Float%20%28single-precision%29))
  ;[0 0 0] Урон
  ;;[0.8695 1 0.9378] Урон исходящий
  (bind _output_get (Variables|Default|SetHealth (- (Variables|Default|GetHealth) Damage)))
  (if (<= _output_get 0.0) ; Чек мертв?
    (bind _astop_down_character (Utilities|Casting|CastToTopDownCharacter (Game|GetPlayerCharacter 0)))
    (Actor|DestroyActor _astop_down_character)))

(event Game|Damage|EventAnyDamage
  (params (Damage :type Float%20%28single-precision%29) (DamageType :type Damage%20Type%20Object%20Reference) (InstigatedBy :type Controller%20Object%20Reference) (DamageCauser :type Actor%20Object%20Reference))
  ;[0 0 0] Урон
  ;;[0.9987 0.9767 1] Входящий урон
  (if (<= (Variables|Default|GetHealth) 0.0)
    (Components|Animation|PlayAnimation (Variables|Character|GetMesh) "/Game/Downloaded/AnimStarterPack/Death_1.Death_1" false)
    (Pawn|Components|CharacterMovement|DisableMovement (Variables|Character|GetCharacterMovement))
    (Physics|SetSimulatePhysics (Variables|Character|GetMesh) false)
    (Utilities|FlowControl|Delay 1e+01)
    (Actor|DestroyActor self)
    (else
      (Audio|PlaySoundatLocation "/Game/Downloaded/Sounds/zombir/Zombie_hit_cue.Zombie_hit_cue" (Transformation|GetWorldLocation (Variables|Character|GetMesh)) "0, 0, 0" 1.0 1.0 0.0 0 0 0))))

(event EventBeginPlay
  (bind _returnvalue (Game|GetPlayerCharacter 0))
  (Utilities|FlowControl|Sequence
    (:then_0
      (Transformation|SetActorRotation (Math|Rotator|MakeRotator 0.0 0.0 (.yaw (Math|Rotator|FindLookatRotation (Transformation|GetActorLocation) (Transformation|GetActorLocation (Game|GetPlayerCharacter 0)))))) ; Искать после спавна
      ;[0 0 0] Преследование
      (AI|AIMoveTo self "0, 0, 0" _returnvalue 5.0 false :!label _label
        (:OnSuccess
          (Game|Damage|ApplyDamage _returnvalue (Variables|Default|GetDamage) 0 self) ; Дамаг по игроку
        )
        (:OnFail
          _))
      (Utilities|FlowControl|Delay 0.2)
      (goto _label))))

(event Game|Damage|EventRadialDamage
  (params (DamageReceived :type Float%20%28single-precision%29) (DamageType :type Damage%20Type%20Object%20Reference) (Origin :type Vector :default "0, 0, 0") (HitInfo :type Hit%20Result%20Structure%20%28by%20ref%29) (InstigatedBy :type Controller%20Object%20Reference) (DamageCauser :type Actor%20Object%20Reference))
  ;[0 0 0] Урон
  ;;[1 0.9393 0.999] АоЕ урон (доработать)
  (CallFunction|ApplyDamage (Variables|Default|GetDamage)))

(fn ConstructionScript)